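; Clyde ghost Blueprint for a Pac-Man game, overriding the parent's chase targeting with his shy behavior.
; BeginPlay caches the first BP_HouseC actor's location as his retreat point.
; SetTargetInChase compares his distance to Pac-Man's TargetPosition against a grid-scaled threshold: at or beyond it he targets one cell ahead of Pac-Man, inside it he retreats to the house.
; Each chosen target is drawn as a debug circle.
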(event `self.ReceiveBeginPlay`
  (`parent.ReceiveBeginPlay`)
  (bind _outactors (`GameplayStatics.GetAllActorsOfClass` "/Game/PacManContent/BluePrint/Ghosts/BP_HouseC.BP_HouseC_C"))
  (bind _output (`|GetArrayItem` _outactors))
  (if (`KismetSystemLibrary.IsValid` _output)
    (set `self.HousePos` (`self.K2_GetActorLocation` _output))))

(fn `SetTargetInChase`
  (returns (targetPos :type "Vector Structure"))
  (bind _pacman (`self.PacMan`))
  (`parent.SetTargetInChase`)
  (if (<= (* (`self.ClydeChaseValue`) (`self.DefaultGridSize`)) (`KismetMathLibrary.Vector_Distance` (`self.K2_GetActorLocation`) (`/Game/PacManContent/BluePrint/BP_PacMan.TargetPosition` _pacman)))
    (bind _output_get (set `self.TargetPosition` (+ (`self.K2_GetActorLocation` _pacman) (* (`/Game/PacManContent/BluePrint/BP_PacMan.CurDir` _pacman) (`self.DefaultGridSize`)))))
    (`KismetSystemLibrary.DrawDebugCircle` _output_get 100.0 12 (`KismetMathLibrary.Conv_ColorToLinearColor` (`self.DebugColor`)) 0.5 10.0 (0.0 1.0 0.0) (1.0 0.0 0.0))
    (return _output_get)
    (else
      (bind _output_get_2 (set `self.TargetPosition` (`self.HousePos`)))
      (`KismetSystemLibrary.DrawDebugCircle` _output_get_2 100.0 12 (`KismetMathLibrary.Conv_ColorToLinearColor` (`self.DebugColor`)) 0.5 10.0 (0.0 1.0 0.0) (1.0 0.0 0.0))
      (return _output_get_2))))

(fn `UserConstructionScript`
  (`parent.UserConstructionScript`))