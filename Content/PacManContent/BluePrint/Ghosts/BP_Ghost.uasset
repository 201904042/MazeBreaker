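; BP_Ghost is a Pac-Man ghost actor that notifies the game mode when it overlaps Pac-Man while chasing or scattering.
; A timer drives activation and Chase/Scatter switching, and the state picks the target: player, own house or main house.
; At each grid cell it snaps, line-traces for Wall-tagged blockers and greedily picks the non-reversing direction nearest that target.
; ChangeState sets material and speed per mode, including Frighten and Eaten.
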(event `self.ReceiveBeginPlay`
  (bind _returnvalue (`Controller.K2_GetPawn` (`GameplayStatics.GetPlayerController` 0)))
  ;[1 1 1] 초기화
  (if (`KismetSystemLibrary.IsValid` _returnvalue)
    (bind _asbp_pac_man (cast `/Game/PacManContent/BluePrint/BP_PacMan` _returnvalue))
    (set `self.PacMan` _asbp_pac_man)
    (bind _asbp_game_mode (cast `/Game/PacManContent/BluePrint/BP_GameMode` (`GameplayStatics.GetGameMode`)))
    (set `self.GameMode` _asbp_game_mode)
    (set `self.ModeTimer` 0.0)))

(event `self.ReceiveActorBeginOverlap`
  (params (OtherActor :type "Actor Object Reference"))
  ;[1 1 1] 충돌 트리거
  (if (== OtherActor (`self.PacMan`))
    (switch `/Game/PacManContent/BluePrint/Ghosts/BP_GhostState` (`self.State`)
      (:`NewEnumerator0`
        _)
      (:`NewEnumerator1`
        _))
    (`/Game/PacManContent/BluePrint/BP_GameMode.PacManCatchedHandler` (`self.GameMode`))))

(event `self.ReceiveTick`
  (params (DeltaSeconds :type "Float (single-precision)"))
  (bind _defaultgridsize (`self.DefaultGridSize`))
  (bind _defaultgridsize_2 (`self.DefaultGridSize`))
  (`self.Mode Timer` DeltaSeconds)
  (if (`/Game/PacManContent/BluePrint/BP_GameMode.IsGameStart` (`self.GameMode`))
    (if (not (`self.OnActive`))
      (`self.CheckOnActive`))
    ;[1 1 1] 맨 처음 입력 세팅
    (if (== (`self.MoveDir`) (`KismetMathLibrary.Vector_Zero`))
      (bind _targetpos (`self.Update Target Pos`))
      (`self.ChangeMoveDir` _targetpos)
      (else
        (if (< (`KismetMathLibrary.Vector_Distance` (`self.K2_GetActorLocation`) (`self.TargetGridPos`)) 10.0)
          (`self.K2_SetActorLocation` (`KismetMathLibrary.MakeVector` (* (`KismetMathLibrary.Round` (/ (.x (`self.K2_GetActorLocation`)) _defaultgridsize_2)) _defaultgridsize) (* (`KismetMathLibrary.Round` (/ (.y (`self.K2_GetActorLocation`)) _defaultgridsize_2)) _defaultgridsize)))
          (bind _targetpos_2 (`self.Update Target Pos`))
          (`self.ChangeMoveDir` _targetpos_2))
        (`self.K2_SetActorLocationAndRotation` (+ (`self.K2_GetActorLocation`) (* (* (`self.MoveDir`) (`self.CurSpeed`)) DeltaSeconds)))))))

(fn `ChangeMoveDir`
  (params (TartetPos :type "Vector Structure"))
  (locals (TargetPos :type "Vector Structure") (DirList :type "Array of Vector Structure") (distanceIndex :type "Float (double-precision)" :default 99999.0) (bestDirIndex :type Integer :default -1))
  (bind _returnvalue (`self.K2_GetActorLocation`))
  (bind _output (`|GetArrayItem` (`local.DirList`) (`local.bestDirIndex`)))
  (set `local.TargetPos` TartetPos)
  (for (_array_element _array_index) (`local.DirList`)
    (if (not (== (* (`self.MoveDir`) (-1.0 -1.0 0.0)) _array_element))
      (bind _outactors (`GameplayStatics.GetAllActorsOfClass` "BP_Ghost_C"))
      (bind _returnvalue_2 (+ _returnvalue (* _array_element (`self.DefaultGridSize`))))
      (bind _outhits (`KismetSystemLibrary.LineTraceMulti` _returnvalue _returnvalue_2 "TraceTypeQuery1" false _outactors))
      (for _array_element_2 _outhits
        (bind (_bblockinghit _binitialoverlap _time _distance _location _impactpoint _normal _impactnormal _physmat _hitactor) (`GameplayStatics.BreakHitResult` _array_element_2))
        (if _bblockinghit
          (if (`self.ActorHasTag` _hitactor "Wall")
            (set `self.isHitWall` true)
            (break)
            (else
              (set `self.isHitWall` false)))))
      (if (`self.isHitWall`)
        (set `self.isHitWall` false)
        (else
          (bind _returnvalue_3 (`KismetMathLibrary.Vector_Distance` _returnvalue_2 (`local.TargetPos`)))
          (if (< _returnvalue_3 (`local.distanceIndex`))
            (set `local.distanceIndex` _returnvalue_3)
            (set `local.bestDirIndex` _array_index))))))
  (set `self.MoveDir` _output)
  (set `self.TargetGridPos` (+ (* _output (`self.DefaultGridSize`)) (`self.K2_GetActorLocation`))))

(fn `ChangeState`
  (params (ChangeState :type "/Game/PacManContent/BluePrint/Ghosts/BP_GhostState Enum" :default "NewEnumerator0"))
  (bind _ghostmesh (`self.ghostMesh`))
  (switch `/Game/PacManContent/BluePrint/Ghosts/BP_GhostState` ChangeState
    (:`NewEnumerator0`
      (`PrimitiveComponent.SetMaterial` _ghostmesh 0 (`self.C_BasicMat`) :!label _label)
      (set `self.CurSpeed` (`self.BasicSpeed`)))
    (:`NewEnumerator1`
      (goto _label))
    (:`NewEnumerator2`
      (`PrimitiveComponent.SetMaterial` _ghostmesh 0 (`self.FrightenMat`))
      (set `self.CurSpeed` (`self.FrightenSpeed`))
      (set `self.FrightenTimer` (`/Game/PacManContent/BluePrint/BP_GameMode.Stage_GhostFrightenTime` (`self.GameMode`))))
    (:`NewEnumerator3`
      (`PrimitiveComponent.SetMaterial` _ghostmesh 0 (`self.EatenMat`))
      (set `self.CurSpeed` (`self.EatenSpeed`)))))

(fn `CheckOnActive`
  (if (not (<= (`self.ModeTimer`) (`self.C_OnActiveTime`)))
    (set `self.OnActive` true)
    (`KismetSystemLibrary.PrintText` "activate" true true (`KismetMathLibrary.Conv_ColorToLinearColor` (`self.C_DebugColor`)))))

(fn `Mode Timer`
  (params (TimeDelta :type "Float (double-precision)"))
  (locals (timeInstance :type "Float (double-precision)" :default 10.0))
  (bind _state (`self.State`))
  (if (or (`|EnumEquality` _state "NewEnumerator0") (`|EnumEquality` _state "NewEnumerator1"))
    (bind _output_get (set `self.ModeTimer` (+ (`self.ModeTimer`) TimeDelta)))
    (if (>= _output_get (`local.timeInstance`))
      (if (`|EnumEquality` (`self.State`) "NewEnumerator0")
        (set `self.State` "NewEnumerator1")
        (else
          (set `self.State` "NewEnumerator0")))
      (set `self.ModeTimer` 10.0))))

(fn `Set Target on Un Active`
  (returns (targetPos :type "Vector Structure"))
  (return (0.0 0.0 0.0)))

(fn `SetTargetInChase`
  (returns (targetPos :type "Vector Structure"))
  (bind _returnvalue (`Controller.K2_GetPawn` (`GameplayStatics.GetPlayerController` 0)))
  (if (`KismetSystemLibrary.IsValid` _returnvalue)
    (bind _output_get (set `self.TargetPosition` (`self.K2_GetActorLocation` _returnvalue)))
    (`KismetSystemLibrary.DrawDebugCircle` _output_get 100.0 12 (`KismetMathLibrary.Conv_ColorToLinearColor` (`self.C_DebugColor`)) 0.5 10.0 (0.0 1.0 0.0) (1.0 0.0 0.0))
    (return _output_get)))

(fn `SetTargetToHome`
  (returns (targetPos :type "Vector Structure"))
  (return (`self.C_HousePos`)))

(fn `SetTargetToMainHome`
  (returns (targetPos :type "Vector Structure"))
  (return (`self.MainHousePos`)))

(fn `Update Target Pos`
  (returns (targetPos :type "Vector Structure"))
  (if (`self.OnActive`)
    (switch `/Game/PacManContent/BluePrint/Ghosts/BP_GhostState` (`self.State`)
      (:`NewEnumerator0`
        (bind _targetpos (`self.SetTargetInChase`))
        (return _targetpos))
      (:`NewEnumerator1`
        _)
      (:`NewEnumerator2`
        _)
      (:`NewEnumerator3`
        (bind _targetpos_2 (`self.SetTargetToMainHome`))
        (return _targetpos_2)))
    (bind _targetpos_3 (`self.SetTargetToHome`))
    (return _targetpos_3)
    (else
      (bind _targetpos_4 (`self.Set Target on Un Active`))
      (return _targetpos_4))))

(fn `UserConstructionScript`)