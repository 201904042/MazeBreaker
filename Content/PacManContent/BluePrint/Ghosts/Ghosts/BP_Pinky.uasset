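; Pinky ghost for a Pac-Man game, a child Blueprint that specializes its parent ghost's setup and chase targeting.
; On BeginPlay it takes its house position from BP_HouseP and, if that actor is valid, starts inactive with a start time and a spawn point at MainHouse's PSpawn.
; SetTargetInChase aims ahead of Pac-Man along his current direction by PinkyChaseValue plus one grid steps, drawing a debug circle there.
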(event `self.ReceiveBeginPlay`
  (bind _mainhouse (`self.MainHouse`))
  (`parent.ReceiveBeginPlay`)
  (bind _outactors (`GameplayStatics.GetAllActorsOfClass` "/Game/PacManContent/BluePrint/Ghosts/HouseTransform/BP_HouseP.BP_HouseP_C"))
  (bind _output (`|GetArrayItem` _outactors))
  (if (`KismetSystemLibrary.IsValid` _output)
    (set `self.C_HousePos` (`self.K2_GetActorLocation` _output))
    (set `self.OnActive` false)
    (set `self.C_OnStartTime` 2.0)
    (set `self.C_SpawnPosition` (+ (`self.K2_GetActorLocation` _mainhouse) (`SceneComponent.RelativeLocation` (`/Game/PacManContent/BluePrint/Ghosts/SpawnTransform/GhostSpawner.PSpawn` _mainhouse))))))

(fn `SetTargetInChase`
  (returns (targetPos :type "Vector Structure"))
  (bind _pacman (`self.PacMan`))
  (bind _returnvalue (* (`/Game/PacManContent/BluePrint/BP_PacMan.CurDir` _pacman) (`self.DefaultGridSize`)))
  (`parent.SetTargetInChase`)
  (bind _output_get (set `self.TargetPosition` (+ (* _returnvalue (`self.PinkyChaseValue`)) (+ _returnvalue (`self.K2_GetActorLocation` _pacman)))))
  (`KismetSystemLibrary.DrawDebugCircle` _output_get 100.0 12 (`KismetMathLibrary.Conv_ColorToLinearColor` (`self.C_DebugColor`)) 0.5 10.0 (0.0 1.0 0.0) (1.0 0.0 0.0))
  (return _output_get))

(fn `UserConstructionScript`
  (`parent.UserConstructionScript`))