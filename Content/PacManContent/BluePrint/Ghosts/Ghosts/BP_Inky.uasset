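; BP_Inky is the Inky ghost Blueprint for a Pac-Man game, extending a parent ghost with its own house and chase targeting.
; BeginPlay caches its house position and a Blinky reference, then starts it inactive with a start time and spawn point in the main house.
; SetTargetInChase point-reflects Blinky's position, offset by its move direction, through a point ahead of Pac-Man, and draws a debug circle at the target.
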(event `self.ReceiveBeginPlay`
  (bind _mainhouse (`self.MainHouse`))
  (`parent.ReceiveBeginPlay`)
  (bind _outactors (`GameplayStatics.GetAllActorsOfClass` "/Game/PacManContent/BluePrint/Ghosts/HouseTransform/BP_HouseI.BP_HouseI_C"))
  (bind _output (`|GetArrayItem` _outactors))
  (if (`KismetSystemLibrary.IsValid` _output)
    (set `self.C_HousePos` (`self.K2_GetActorLocation` _output))
    (bind _outactors_2 (`GameplayStatics.GetAllActorsOfClass` "/Game/PacManContent/BluePrint/Ghosts/Ghosts/BP_Blinky.BP_Blinky_C"))
    (bind _output_2 (`|GetArrayItem` _outactors_2))
    (if (`KismetSystemLibrary.IsValid` _output_2)
      (set `self.Blinky` _output_2)
      (set `self.OnActive` false)
      (set `self.C_OnStartTime` 5.0)
      (set `self.C_SpawnPosition` (+ (`self.K2_GetActorLocation` _mainhouse) (`SceneComponent.RelativeLocation` (`/Game/PacManContent/BluePrint/Ghosts/SpawnTransform/GhostSpawner.ISpawn` _mainhouse)))))))

(fn `SetTargetInChase`
  (returns (targetPos :type "Vector Structure"))
  (locals (centerPoint :type "Vector Structure"))
  (bind _pacman (`self.PacMan`))
  (bind _blinky (`self.Blinky`))
  (`parent.SetTargetInChase`)
  ;[1 1 1] 팩맨의 진행방향 2칸 앞을 구함 = 회전대칭의  중심
  (set `local.centerPoint` (+ (* (* (`/Game/PacManContent/BluePrint/BP_PacMan.CurDir` _pacman) (`self.DefaultGridSize`)) (`self.InkyChaseValue`)) (`self.K2_GetActorLocation` _pacman)))
  (bind _output_get (set `self.TargetPosition` (`KismetMathLibrary.MakeVector` (- (* (.x (`local.centerPoint`)) 2.0) (.x (+ (`self.K2_GetActorLocation` _blinky) (* (`/Game/PacManContent/BluePrint/Ghosts/BP_Ghost.MoveDir` _blinky) (`self.DefaultGridSize`))))) (- (* (.y (`local.centerPoint`)) 2.0) (.y (+ (`self.K2_GetActorLocation` _blinky) (* (`/Game/PacManContent/BluePrint/Ghosts/BP_Ghost.MoveDir` _blinky) (`self.DefaultGridSize`))))))))
  (`KismetSystemLibrary.DrawDebugCircle` _output_get 100.0 12 (`KismetMathLibrary.Conv_ColorToLinearColor` (`self.C_DebugColor`)) 0.5 10.0 (0.0 1.0 0.0) (1.0 0.0 0.0))
  (return _output_get))

(fn `UserConstructionScript`
  (`parent.UserConstructionScript`))