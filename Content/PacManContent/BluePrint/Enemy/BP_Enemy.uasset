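; BP_Enemy is a Pac-Man style ghost that chases the player on a grid and notifies BP_GameMode when it touches them while chasing.
; A state enum gates movement, with a Tick timer switching Respawn to Chase.
; At each cell it snaps to the grid, line-traces for tagged walls and greedily picks the open direction nearest the player, normally excluding reversal.
; ChangeAnim is an empty hook called on state changes.
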(event `self.ReceiveBeginPlay`
  (bind _returnvalue (`Controller.K2_GetPawn` (`GameplayStatics.GetPlayerController` 0)))
  ;[1 1 1] 초기화
  (if (`KismetSystemLibrary.IsValid` _returnvalue)
    (bind _asbp_new_player (cast `/Game/PacManContent/BluePrint/FirstPersonPlayer/FirstPerson/Blueprints/BP_NewPlayer` _returnvalue))
    (set `self.Player` _asbp_new_player)
    (bind _asbp_game_mode (cast `/Game/PacManContent/BluePrint/BP_GameMode` (`GameplayStatics.GetGameMode`)))
    (set `self.GameMode` _asbp_game_mode)
    (`self.Init`)))

(event `self.ReceiveActorBeginOverlap`
  (params (OtherActor :type "Actor Object Reference"))
  ;[1 1 1] 충돌 트리거
  (if (== OtherActor (`self.Player`))
    (if (`|EnumEquality` (`self.State`) "NewEnumerator0")
      (`/Game/PacManContent/BluePrint/BP_GameMode.PlayerCatched` (`self.GameMode`) self))))

(event `self.ReceiveTick`
  (params (DeltaSeconds :type "Float (single-precision)"))
  (`self.TimerAction` DeltaSeconds)
  (if (`self.OnActive`)
    ;[1 1 1] 맨 처음 입력 세팅
    (if (== (`self.MoveDir`) (`KismetMathLibrary.Vector_Zero`))
      (bind _targetpos (`self.SetTargetInChase`))
      (`self.ChangeMoveDir` _targetpos))
    (`self.Move To Target` DeltaSeconds)))

(fn `ChangeAnim`
  (params (state :type "/Game/PacManContent/BluePrint/Enemy/BP_EnemyState Enum" :default "NewEnumerator0")))

(fn `ChangeMoveDir`
  (params (TartetPos :type "Vector Structure"))
  (locals (TargetPos :type "Vector Structure") (DirList :type "Array of Vector Structure") (distanceIndex :type "Float (double-precision)" :default 99999.0) (bestDirIndex :type Integer :default -1))
  (bind _returnvalue (`self.K2_GetActorLocation`))
  (bind _output (`|GetArrayItem` (`local.DirList`) (`local.bestDirIndex`)))
  (bind _output_get (set `local.TargetPos` TartetPos))
  (`KismetSystemLibrary.DrawDebugCircle` _output_get 100.0 12 (`KismetMathLibrary.Conv_ColorToLinearColor` (`self.C_DebugColor`)) 0.5 10.0 (0.0 1.0 0.0) (1.0 0.0 0.0))
  (for (_array_element _array_index) (`local.DirList`)
    ;[1 1 1] 활성화 전 상태에서는 위의 체크가 필요 없음
    (if true
      ;[1 1 1] 상태가 바뀐 후 한번에 한해 진행방향의 뒷방향 이동 허용함
      (if (`self.IsAbleToMoveBack`)
        (set `self.IsAbleToMoveBack` false)
        (bind _returnvalue_2 (+ _returnvalue (* _array_element (`self.DefaultGridSize`))))
        (bind _outhits (`KismetSystemLibrary.LineTraceMulti` :`Start` _returnvalue :`End` _returnvalue_2 :`TraceChannel` "TraceTypeQuery1" :`bTraceComplex` true :`DrawTime` 1.0 :!label _label))
        (for _array_element_2 _outhits
          (bind (_bblockinghit _binitialoverlap _time _distance _location _impactpoint _normal _impactnormal _physmat _hitactor) (`GameplayStatics.BreakHitResult` _array_element_2))
          ;[1 1 1] 진행방향에 벽이 있는지 체크
          (if _bblockinghit
            (if (`self.ActorHasTag` _hitactor "Wall")
              (set `self.WallHit` true :!label _label_2)
              (break)
              (elif true
                (if (`self.ActorHasTag` _hitactor "EntranceWall")
                  (goto _label_2))))))
        ;[1 1 1] 벽이 없다면 해당 방향으로 설정함
        (if (`self.WallHit`)
          (set `self.WallHit` false)
          (else
            (bind _returnvalue_3 (`KismetMathLibrary.Vector_Distance` _returnvalue_2 (`local.TargetPos`)))
            (if (< _returnvalue_3 (`local.distanceIndex`))
              (set `local.distanceIndex` _returnvalue_3)
              (set `local.bestDirIndex` _array_index))))
        (elif (not (== (* (`self.MoveDir`) (-1.0 -1.0 0.0)) _array_element))
          (goto _label)))
      (else
        (goto _label))))
  ;[1 1 1] 최적의 방향을 통해 타겟위치를 설정
  (set `self.MoveDir` _output)
  (set `self.MovePos` (+ (* _output (`self.DefaultGridSize`)) (`self.K2_GetActorLocation`))))

(fn `ChangeState`
  (params (ChangeState :type "/Game/PacManContent/BluePrint/Enemy/BP_EnemyState Enum" :default "NewEnumerator0"))
  (bind _output_get (set `self.State` ChangeState))
  (switch `/Game/PacManContent/BluePrint/Enemy/BP_EnemyState` _output_get
    (:`NewEnumerator0`
      (`KismetSystemLibrary.PrintString` "추격")
      (set `self.OnActive` true))
    (:`NewEnumerator1`
      (`KismetSystemLibrary.PrintString` "사망")
      (set `self.OnActive` false :!label _label))
    (:`NewEnumerator2`
      (`KismetSystemLibrary.PrintString` "재생성")
      (goto _label))
    (:`NewEnumerator4`
      (`KismetSystemLibrary.PrintString` "기절")
      (goto _label)))
  (`self.ChangeAnim` ChangeState))

(fn `Init`
  (bind _returnvalue (`self.K2_GetActorLocation`))
  (set `self.TargetPosition` _returnvalue)
  (set `self.MovePos` _returnvalue)
  (set `self.MoveDir` (0.0 0.0 0.0))
  (set `self.OnActive` false)
  (set `self.WallHit` false)
  (set `self.IsAbleToMoveBack` false)
  (set `self.CurSpeed` (`self.BasicSpeed`))
  (set `self.OnStartTimer` 0.0)
  (`self.ChangeState` "NewEnumerator2"))

(fn `Move To Target`
  (params (delta :type "Float (double-precision)"))
  (bind _returnvalue (`self.K2_GetActorLocation`))
  (bind _defaultgridsize (`self.DefaultGridSize`))
  (bind _defaultgridsize_2 (`self.DefaultGridSize`))
  (if (< (`KismetMathLibrary.Vector_Distance` (`self.K2_GetActorLocation`) (`self.MovePos`)) 10.0)
    (`self.K2_SetActorLocation` (`KismetMathLibrary.MakeVector` (* (`KismetMathLibrary.Round` (/ (.x (`self.K2_GetActorLocation`)) _defaultgridsize_2)) _defaultgridsize) (* (`KismetMathLibrary.Round` (/ (.y (`self.K2_GetActorLocation`)) _defaultgridsize_2)) _defaultgridsize)))
    (bind _targetpos (`self.SetTargetInChase`))
    (`self.ChangeMoveDir` _targetpos))
  (`self.K2_SetActorLocationAndRotation` (+ _returnvalue (* (* (`self.MoveDir`) (`self.CurSpeed`)) delta)) (`KismetMathLibrary.RInterpTo` (`self.K2_GetActorRotation`) (`KismetMathLibrary.FindLookAtRotation` _returnvalue (`self.MovePos`)) delta 15.0)))

(fn `SetTargetInChase`
  (returns (targetPos :type "Vector Structure"))
  (bind _returnvalue (`Controller.K2_GetPawn` (`GameplayStatics.GetPlayerController` 0)))
  (if (`KismetSystemLibrary.IsValid` _returnvalue)
    (bind _output_get (set `self.TargetPosition` (`self.K2_GetActorLocation` _returnvalue)))
    (return _output_get)))

(fn `TimerAction`
  (params (delta :type "Float (double-precision)"))
  (if (`|EnumEquality` (`self.State`) "NewEnumerator2")
    ;[1 1 1] 유령이 스테이지에서 시작하기까지의 타이머
    (if (not (`self.OnActive`))
      (bind _output_get (set `self.OnStartTimer` (+ delta (`self.OnStartTimer`))))
      (if (> _output_get 3.0)
        (`self.ChangeState` "NewEnumerator0")))))

(fn `UserConstructionScript`)