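; BP_Clyde is the Clyde ghost enemy for a Pac-Man game, acting as a guard of its spawn point.
; In one state, it targets the player when they are within a grid-cell radius of that spawn, otherwise returning there to wait.
; Tick drives grid-snapped movement with interpolated turning and ABP_Clyde animation states, drawing debug circles at chase targets.
; On destruction it clears its reference on the owning BP_CornorSpawnPoint.
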(event `self.ReceiveBeginPlay`
  (`parent.ReceiveBeginPlay`))

(event `self.ReceiveTick`
  (params (DeltaSeconds :type "Float (single-precision)"))
  (`self.TimerAction` DeltaSeconds)
  (`self.CheckClyde`)
  (if (`self.OnActive`)
    (`self.Move to Target` DeltaSeconds)))

(fn `ChangeAnim`
  (params (state :type "/Game/PacManContent/BluePrint/Enemy/BP_EnemyState Enum" :default "NewEnumerator0"))
  (bind _enemymesh (`self.EnemyMesh`))
  (`parent.ChangeAnim` state)
  (`SkeletalMeshComponent.SetAnimInstanceClass` _enemymesh "/Game/PacManContent/BluePrint/Enemy/ABP/ABP_Clyde.ABP_Clyde_C")
  (bind _asabp_clyde (cast `/Game/PacManContent/BluePrint/Enemy/ABP/ABP_Clyde` (`SkeletalMeshComponent.GetAnimInstance` _enemymesh))
    (:`then`
      (set `/Game/PacManContent/BluePrint/Enemy/ABP/ABP_Clyde.curState` state _asabp_clyde))
    (:`CastFailed`
      (`KismetSystemLibrary.PrintString` "애니메이션 로드 실패"))))

(fn `CheckClyde`
  (if (`|EnumEquality` (`self.State`) "NewEnumerator0")
    (if (>= (* (`self.ClydeChaseValue`) (`self.DefaultGridSize`)) (`KismetMathLibrary.Vector_Distance` (`self.SpawnPosition`) (`self.K2_GetActorLocation` (`self.Player`))))
      (set `self.IsPlayerInRange` true)
      (else
        (set `self.IsPlayerInRange` false)
        (if (== (`self.SpawnPosition`) (`self.K2_GetActorLocation`) :`ErrorTolerance` 10.0)
          (set `self.IsClydeOnSpawnPoint` true)
          (else
            (set `self.IsClydeOnSpawnPoint` false)))))))

(fn `EnemyDestroyHandler`
  (bind _asbp_cornor_spawn_point (cast `/Game/PacManContent/BluePrint/Enemy/SpawnPoint/BP_CornorSpawnPoint` (`self.SpawnActor`)))
  (set `/Game/PacManContent/BluePrint/Enemy/SpawnPoint/BP_CornorSpawnPoint.SpawnClyde` null _asbp_cornor_spawn_point)
  (`parent.EnemyDestroyHandler`))

(fn `Move to Target`
  (params (delta :type "Float (double-precision)"))
  (bind _returnvalue (`self.K2_GetActorLocation`))
  (bind _defaultgridsize (`self.DefaultGridSize`))
  (bind _defaultgridsize_2 (`self.DefaultGridSize`))
  (`self.ChangeAnim` "NewEnumerator0")
  (if (< (`KismetMathLibrary.Vector_Distance` (`self.K2_GetActorLocation`) (`self.MovePos`)) 10.0)
    (`self.K2_SetActorLocation` (`KismetMathLibrary.MakeVector` (* (`KismetMathLibrary.Round` (/ (.x (`self.K2_GetActorLocation`)) _defaultgridsize_2)) _defaultgridsize) (* (`KismetMathLibrary.Round` (/ (.y (`self.K2_GetActorLocation`)) _defaultgridsize_2)) _defaultgridsize)))
    (if (`self.IsPlayerInRange`)
      (bind _targetpos (`self.SetTargetInChase` :!label _label))
      (`self.ChangeMoveDir` _targetpos)
      (`self.K2_SetActorLocationAndRotation` (+ _returnvalue (* (* (`self.MoveDir`) (`self.CurSpeed`)) delta)) (`KismetMathLibrary.RInterpTo` (`self.K2_GetActorRotation`) (`KismetMathLibrary.FindLookAtRotation` _returnvalue (`self.MovePos`)) delta 15.0) :!label _label_2)
      (elif (`self.IsClydeOnSpawnPoint`)
        (`self.ChangeAnim` "NewEnumerator2")
        (`self.K2_SetActorRotation` (`SceneComponent.K2_GetComponentRotation` (`Actor.RootComponent` (`self.SpawnActor`))))
        (else
          (goto _label))))
    (else
      (goto _label_2))))

(fn `SetTargetInChase`
  (returns (targetPos :type "Vector Structure"))
  (`parent.SetTargetInChase`)
  (if (`self.IsPlayerInRange`)
    (bind _output_get (set `self.TargetPosition` (`self.K2_GetActorLocation` (`self.Player`))))
    (`KismetSystemLibrary.DrawDebugCircle` _output_get 100.0 12 (`KismetMathLibrary.Conv_ColorToLinearColor` (`self.C_DebugColor`)) 0.5 10.0 (0.0 1.0 0.0) (1.0 0.0 0.0))
    (return _output_get)
    (else
      (bind _output_get_2 (set `self.TargetPosition` (`self.SpawnPosition`)))
      (`KismetSystemLibrary.DrawDebugCircle` _output_get_2 100.0 12 (`KismetMathLibrary.Conv_ColorToLinearColor` (`self.C_DebugColor`)) 0.5 10.0 (0.0 1.0 0.0) (1.0 0.0 0.0))
      (return _output_get_2))))

(fn `UserConstructionScript`
  (`parent.UserConstructionScript`))