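; Inky ghost enemy for a Pac-Man game, overriding its parent's chase targeting and animation hooks.
; Chase targeting takes a point ahead of the player and reflects the selected Blinky's position through it, using a nearest-to-player search bounded by DistanceIndex.
; Without a valid Blinky it targets the point ahead; both cases draw a debug circle.
; Animation changes assign ABP_Inky to the mesh and pass it the new state.
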(event `self.ReceiveBeginPlay`
  (`parent.ReceiveBeginPlay`))

(fn `ChangeAnim`
  (params (state :type "/Game/PacManContent/BluePrint/Enemy/BP_EnemyState Enum" :default "NewEnumerator0"))
  (bind _enemymesh (`self.EnemyMesh`))
  (`parent.ChangeAnim` state)
  (`SkeletalMeshComponent.SetAnimInstanceClass` _enemymesh "/Game/PacManContent/BluePrint/Enemy/ABP/ABP_Inky.ABP_Inky_C")
  (bind _asabp_inky (cast `/Game/PacManContent/BluePrint/Enemy/ABP/ABP_Inky` (`SkeletalMeshComponent.GetAnimInstance` _enemymesh))
    (:`then`
      (set `/Game/PacManContent/BluePrint/Enemy/ABP/ABP_Inky.curState` state _asabp_inky))
    (:`CastFailed`
      (`KismetSystemLibrary.PrintString` "애니메이션 로드 실패"))))

(fn `SetTargetInChase`
  (returns (targetPos :type "Vector Structure"))
  (locals (centerPoint :type "Vector Structure") (distanceIndex :type "Float (double-precision)" :default 99999.0))
  (bind _player (`self.Player`))
  (`parent.SetTargetInChase`)
  ;[1 1 1] 팩맨의 진행방향 2칸 앞을 구함 = 회전대칭의  중심
  (bind _output_get (set `local.centerPoint` (+ (* (* (`self.GetActorForwardVector` _player) (`self.DefaultGridSize`)) (`self.InkyChaseValue`)) (`self.K2_GetActorLocation` _player))))
  (bind _outactors (`GameplayStatics.GetAllActorsOfClass` "/Game/PacManContent/BluePrint/Enemy/Enemys/BP_Blinky.BP_Blinky_C"))
  (for _array_element _outactors
    (bind _returnvalue (`KismetMathLibrary.Vector_Distance` (`self.K2_GetActorLocation` _array_element) (`self.K2_GetActorLocation` (`self.Player`))))
    (if (< _returnvalue (`local.distanceIndex`))
      (set `local.distanceIndex` _returnvalue)
      (set `self.BlinkyTarget` _array_element)))
  (if (`KismetSystemLibrary.IsValid` (`self.BlinkyTarget`))
    (bind _output_get_2 (set `self.TargetPosition` (`KismetMathLibrary.MakeVector` (- (* (.x (`local.centerPoint`)) 2.0) (.x (`self.K2_GetActorLocation` (`self.BlinkyTarget`)))) (- (* (.y (`local.centerPoint`)) 2.0) (.y (`self.K2_GetActorLocation` (`self.BlinkyTarget`)))))))
    (`KismetSystemLibrary.DrawDebugCircle` _output_get_2 100.0 12 (`KismetMathLibrary.Conv_ColorToLinearColor` (`self.C_DebugColor`)) 0.5 10.0 (0.0 1.0 0.0) (1.0 0.0 0.0))
    (return _output_get_2)
    (else
      (bind _output_get_3 (set `self.TargetPosition` _output_get))
      (`KismetSystemLibrary.DrawDebugCircle` _output_get_3 100.0 12 (`KismetMathLibrary.Conv_ColorToLinearColor` (`self.C_DebugColor`)) 0.5 10.0 (0.0 1.0 0.0) (1.0 0.0 0.0))
      (return _output_get_3))))

(fn `UserConstructionScript`
  (`parent.UserConstructionScript`))