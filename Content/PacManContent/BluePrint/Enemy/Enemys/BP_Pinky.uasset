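; BP_Pinky is the Pinky enemy in a Pac-Man game, a child Blueprint that supplies its own chase targeting.
; Its SetTargetInChase override projects the target ahead of the player along their forward vector, by one grid cell plus PinkyChaseValue cells.
; It draws a debug circle at that point.
; An unconnected variant based on the actor's own CurDir and location never runs.
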(event `self.ReceiveBeginPlay`
  (`parent.ReceiveBeginPlay`))

(fn `SetTargetInChase`
  (returns (targetPos :type "Vector Structure"))
  (bind _player (`self.Player`))
  (bind _returnvalue (* (`self.GetActorForwardVector` _player) (`self.DefaultGridSize`)))
  (`parent.SetTargetInChase`)
  (bind _output_get (set `self.TargetPosition` (+ (* _returnvalue (`self.PinkyChaseValue`)) (+ _returnvalue (`self.K2_GetActorLocation` _player)))))
  (`KismetSystemLibrary.DrawDebugCircle` _output_get 100.0 12 (`KismetMathLibrary.Conv_ColorToLinearColor` (`self.C_DebugColor`)) 0.5 10.0 (0.0 1.0 0.0) (1.0 0.0 0.0))
  (return _output_get))

(fn `UserConstructionScript`
  (`parent.UserConstructionScript`))