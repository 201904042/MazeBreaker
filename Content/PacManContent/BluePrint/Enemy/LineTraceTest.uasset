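; LineTraceTest is a debug Blueprint that shows which actors lie along a line from its own location.
; Every Tick it runs a complex multi line trace on the Visibility channel along world +X, drawn for one frame.
; For each hit it prints the index with a Korean ordinal label, then prints every tag on the hit actor.
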(event `self.ReceiveTick`
  (params (DeltaSeconds :type "Float (single-precision)"))
  (bind _returnvalue (`self.K2_GetActorLocation`))
  (bind _outhits (`KismetSystemLibrary.LineTraceMulti` :`Start` _returnvalue :`End` (+ _returnvalue (10000.0 0.0 0.0)) :`TraceChannel` "TraceTypeQuery1" :`bTraceComplex` true :`DrawDebugType` "ForOneFrame"))
  (for (_array_element _array_index) _outhits
    (`KismetSystemLibrary.PrintString` (`KismetStringLibrary.Concat_StrStr` (`KismetStringLibrary.Conv_IntToString` _array_index) (`self.번째 액터`)))
    (for _array_element_2 (`Actor.Tags` (`.HitActor` (`GameplayStatics.BreakHitResult` _array_element)))
      (`KismetSystemLibrary.PrintString` (`KismetStringLibrary.Conv_NameToString` _array_element_2)))))

(fn `UserConstructionScript`)