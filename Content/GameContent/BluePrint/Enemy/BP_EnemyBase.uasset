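; Base Pac-Man ghost that waits on a start timer, heads to the GhostSpawner to activate, then roams the maze.
; State picks target, material and speed: Chase follows the player, Scatter goes home, Frighten wanders randomly, Eaten returns to the spawner to revert.
; Each grid step snaps position and greedily picks the trace-checked direction closest to target, barring reversal except after state changes.
; Player overlaps are forwarded to BP_GameMode.
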(event `self.ReceiveBeginPlay`
  (bind _returnvalue (`Controller.K2_GetPawn` (`GameplayStatics.GetPlayerController` 0)))
  ;[1 1 1] 초기화
  (if (`KismetSystemLibrary.IsValid` _returnvalue)
    (bind _asbp_pac_man (cast `/Game/PacManContent/BluePrint/BP_PacMan` _returnvalue))
    (set `self.PacMan` _asbp_pac_man)
    (bind _asbp_game_mode (cast `/Game/PacManContent/BluePrint/BP_GameMode` (`GameplayStatics.GetGameMode`)))
    (set `self.GameMode` _asbp_game_mode)
    (bind _returnvalue_2 (`GameplayStatics.GetActorOfClass` "/Game/PacManContent/BluePrint/Enemy/SpawnTransform/GhostSpawner.GhostSpawner_C"))
    (set `self.MainHouse` _returnvalue_2)
    (set `self.OnStartTimer` 0.0)))

(event `self.ReceiveActorBeginOverlap`
  (params (OtherActor :type "Actor Object Reference"))
  ;[1 1 1] 충돌 트리거
  (if (== OtherActor (`self.PacMan`))
    (`/Game/PacManContent/BluePrint/BP_GameMode.Overlap Ghost to Pac` (`self.GameMode`) self))
  (if (`self.ActorHasTag` OtherActor "Wall")
    (`KismetSystemLibrary.PrintString` "벽과 겹침" true true (`KismetMathLibrary.Conv_ColorToLinearColor` (`self.C_DebugColor`)))))

(event `self.ReceiveTick`
  (params (DeltaSeconds :type "Float (single-precision)"))
  (if (`/Game/PacManContent/BluePrint/BP_GameMode.IsStageStart` (`self.GameMode`))
    (`self.TimerAction` DeltaSeconds)
    (if (`/Game/PacManContent/BluePrint/BP_GameMode.IsGameStart` (`self.GameMode`))
      (if (not (`self.IsStart`))
        (`self.CheckIsStart`))
      ;[1 1 1] 맨 처음 입력 세팅
      (if (== (`self.MoveDir`) (`KismetMathLibrary.Vector_Zero`))
        (bind _targetpos (`self.Update Target Pos`))
        (`self.ChangeMoveDir` _targetpos))
      (`self.Move To Target` DeltaSeconds))))

(fn `ChangeMoveDir`
  (params (TartetPos :type "Vector Structure"))
  (locals (TargetPos :type "Vector Structure") (DirList :type "Array of Vector Structure") (distanceIndex :type "Float (double-precision)" :default 99999.0) (bestDirIndex :type Integer :default -1))
  (bind _returnvalue (`self.K2_GetActorLocation`))
  (bind _output (`|GetArrayItem` (`local.DirList`) (`local.bestDirIndex`)))
  (bind _output_get (set `local.TargetPos` TartetPos))
  (`KismetSystemLibrary.DrawDebugCircle` _output_get 100.0 12 (`KismetMathLibrary.Conv_ColorToLinearColor` (`self.C_DebugColor`)) 0.5 10.0 (0.0 1.0 0.0) (1.0 0.0 0.0))
  (for (_array_element _array_index) (`local.DirList`)
    ;[1 1 1] 활성화 전 상태에서는 위의 체크가 필요 없음
    (if (`self.OnActive`)
      ;[1 1 1] 상태가 바뀐 후 한번에 한해 진행방향의 뒷방향 이동 허용함
      (if (`self.IsAbleToMoveBack`)
        (set `self.IsAbleToMoveBack` false)
        (bind _returnvalue_2 (+ _returnvalue (* _array_element (`self.DefaultGridSize`))))
        (bind _outhits (`KismetSystemLibrary.LineTraceMulti` :`Start` _returnvalue :`End` _returnvalue_2 :`TraceChannel` "TraceTypeQuery1" :`bTraceComplex` true :`DrawTime` 1.0 :!label _label))
        (for _array_element_2 _outhits
          (bind (_bblockinghit _binitialoverlap _time _distance _location _impactpoint _normal _impactnormal _physmat _hitactor) (`GameplayStatics.BreakHitResult` _array_element_2))
          ;[1 1 1] 진행방향에 벽이 있는지 체크
          (if _bblockinghit
            (if (`self.ActorHasTag` _hitactor "Wall")
              (set `self.WallHit` true :!label _label_2)
              (break)
              (elif (`self.OnActive`)
                (if (`self.ActorHasTag` _hitactor "EntranceWall")
                  (goto _label_2))))))
        ;[1 1 1] 벽이 없다면 해당 방향으로 설정함
        (if (`self.WallHit`)
          (set `self.WallHit` false)
          (else
            (bind _returnvalue_3 (`KismetMathLibrary.Vector_Distance` _returnvalue_2 (`local.TargetPos`)))
            (if (< _returnvalue_3 (`local.distanceIndex`))
              (set `local.distanceIndex` _returnvalue_3)
              (set `local.bestDirIndex` _array_index))))
        (elif (not (== (* (`self.MoveDir`) (-1.0 -1.0 0.0)) _array_element))
          (goto _label)))
      (else
        (goto _label))))
  ;[1 1 1] 최적의 방향을 통해 타겟위치를 설정
  (set `self.MoveDir` _output)
  (set `self.TargetGridPos` (+ (* _output (`self.DefaultGridSize`)) (`self.K2_GetActorLocation`))))

(fn `ChangeState`
  (params (ChangeState :type "/Game/PacManContent/BluePrint/Enemy/BP_EnemyStates Enum" :default "NewEnumerator0"))
  (bind _ghostmesh (`self.ghostMesh`))
  (bind _output_get (set `self.State` ChangeState))
  (switch `/Game/PacManContent/BluePrint/Enemy/BP_EnemyStates` _output_get
    (:`NewEnumerator0`
      (`PrimitiveComponent.SetMaterial` _ghostmesh 0 (`self.C_BasicMat`) :!label _label)
      (set `self.CurSpeed` (`self.BasicSpeed`)))
    (:`NewEnumerator1`
      (goto _label))
    (:`NewEnumerator2`
      (`PrimitiveComponent.SetMaterial` _ghostmesh 0 (`self.FrightenMat`))
      (set `self.CurSpeed` (`self.FrightenSpeed`)))
    (:`NewEnumerator3`
      (`PrimitiveComponent.SetMaterial` _ghostmesh 0 (`self.C_EatenMat`))
      (set `self.CurSpeed` (`self.EatenSpeed`))))
  (set `self.IsAbleToMoveBack` true))

(fn `CheckIsStart`
  (if (> (`self.OnStartTimer`) (`self.C_OnStartTime`))
    (set `self.IsStart` true)
    (`KismetSystemLibrary.PrintText` "Start" true true (`KismetMathLibrary.Conv_ColorToLinearColor` (`self.C_DebugColor`)))
    (set `self.OnStartTimer` 0.0)))

(fn `Init`
  (bind _returnvalue (`self.K2_GetActorLocation`))
  (set `self.TargetPosition` _returnvalue)
  (set `self.TargetGridPos` _returnvalue)
  (set `self.MoveDir` (0.0 0.0 0.0))
  (set `self.WallHit` false)
  (set `self.IsAbleToMoveBack` false)
  (set `self.IsStart` false)
  (set `self.OnActive` false)
  (set `self.Phase` 0)
  (set `self.CurSpeed` (`self.BasicSpeed`))
  (set `self.OnStartTimer` 0.0)
  (`self.ChangeState` (`/Game/PacManContent/BluePrint/BP_GameMode.Stage_CommonGhostState` (`self.GameMode`))))

(fn `Move To Target`
  (params (delta :type "Float (double-precision)"))
  (bind _defaultgridsize (`self.DefaultGridSize`))
  (bind _defaultgridsize_2 (`self.DefaultGridSize`))
  (bind _returnvalue (`KismetMathLibrary.MakeVector` (* (`KismetMathLibrary.Round` (/ (.x (`self.K2_GetActorLocation`)) _defaultgridsize_2)) _defaultgridsize) (* (`KismetMathLibrary.Round` (/ (.y (`self.K2_GetActorLocation`)) _defaultgridsize_2)) _defaultgridsize)))
  (bind _returnvalue_2 (== _returnvalue (`self.K2_GetActorLocation` (`self.MainHouse`)) :`ErrorTolerance` 10.0))
  (if (< (`KismetMathLibrary.Vector_Distance` (`self.K2_GetActorLocation`) (`self.TargetGridPos`)) 10.0)
    (`self.K2_SetActorLocation` _returnvalue)
    (if (`self.IsStart`)
      (if (`self.OnActive`)
        (switch `/Game/PacManContent/BluePrint/Enemy/BP_EnemyStates` (`self.State`)
          (:`NewEnumerator0`
            _)
          (:`NewEnumerator1`
            _)
          (:`NewEnumerator2`
            _)
          (:`NewEnumerator3`
            (if _returnvalue_2
              (`self.ChangeState` (`/Game/PacManContent/BluePrint/BP_GameMode.Stage_CommonGhostState` (`self.GameMode`))))))
        (elif _returnvalue_2
          (set `self.OnActive` true))))
    (bind _targetpos (`self.Update Target Pos`))
    (`self.ChangeMoveDir` _targetpos))
  (`self.K2_SetActorLocationAndRotation` (+ (`self.K2_GetActorLocation`) (* (* (`self.MoveDir`) (`self.CurSpeed`)) delta))))

(fn `Set Target on Un Active`
  (returns (targetPos :type "Vector Structure"))
  (bind _c_spawnposition (`self.C_SpawnPosition`))
  (if (== _c_spawnposition (`self.K2_GetActorLocation`))
    (bind _output_get (set `self.TargetPosition` (`KismetMathLibrary.MakeVector` (+ (.x _c_spawnposition) 100.0) (.y _c_spawnposition) (.z _c_spawnposition))))
    (return _output_get)
    (else
      (bind _output_get_2 (set `self.TargetPosition` (`self.C_SpawnPosition`)))
      (return _output_get_2))))

(fn `SetLocationToSpawnPos`
  (`self.K2_SetActorLocation` (`self.C_SpawnPosition`))
  (`self.Init`))

(fn `SetTargetInChase`
  (returns (targetPos :type "Vector Structure"))
  (bind _returnvalue (`Controller.K2_GetPawn` (`GameplayStatics.GetPlayerController` 0)))
  (if (`KismetSystemLibrary.IsValid` _returnvalue)
    (bind _output_get (set `self.TargetPosition` (`self.K2_GetActorLocation` _returnvalue)))
    (return _output_get)))

(fn `SetTargetToHome`
  (returns (targetPos :type "Vector Structure"))
  (bind _output_get (set `self.TargetPosition` (`self.C_HousePos`)))
  (return _output_get))

(fn `SetTargetToRandom`
  (returns (targetPos :type "Vector Structure"))
  (locals (DirList :type "Array of Vector Structure"))
  (bind _output_get (set `self.TargetPosition` (+ (* (`|GetArrayItem` (`local.DirList`) (`KismetMathLibrary.RandomIntegerInRange` 0 3)) (`self.DefaultGridSize`)) (`self.K2_GetActorLocation`))))
  (return _output_get))

(fn `SetTargetToRespawn`
  (returns (targetPos :type "Vector Structure"))
  (bind _output_get (set `self.TargetPosition` (`self.K2_GetActorLocation` (`self.MainHouse`))))
  (return _output_get))

(fn `TimerAction`
  (params (delta :type "Float (double-precision)"))
  ;[1 1 1] 유령이 스테이지에서 시작하기까지의 타이머
  (if (not (`self.IsStart`))
    (set `self.OnStartTimer` (+ delta (`self.OnStartTimer`)))))

(fn `Update Target Pos`
  (returns (targetPos :type "Vector Structure"))
  (if (`self.IsStart`)
    (if (`self.OnActive`)
      (switch `/Game/PacManContent/BluePrint/Enemy/BP_EnemyStates` (`self.State`)
        (:`NewEnumerator0`
          (bind _targetpos (`self.SetTargetInChase`))
          (return _targetpos))
        (:`NewEnumerator1`
          (bind _targetpos_2 (`self.SetTargetToHome`))
          (return _targetpos_2))
        (:`NewEnumerator2`
          (bind _targetpos_3 (`self.SetTargetToRandom`))
          (return _targetpos_3))
        (:`NewEnumerator3`
          _)))
    (bind _targetpos_4 (`self.SetTargetToRespawn`))
    (return _targetpos_4)
    (else
      (bind _targetpos_5 (`self.Set Target on Un Active`))
      (return _targetpos_5))))

(fn `UserConstructionScript`)