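; BP_PacMan is the Pac-Man player actor, moving on a grid and triggering ItemEaten on overlapped items.
; Enhanced Input axes set a buffered next direction, vertical taking priority, and flag the stage as started in BP_GameMode.
; Tick moves it toward the next cell, snapping to the grid on arrival.
; Line traces for Wall and EntranceWall tags decide whether it turns, continues or stops.
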(event `EnhancedInput|/Game/PacManContent/Input/IA_Horizontal`
  (params (ActionValue :type "Float (double-precision)") (ElapsedSeconds :type "Float (double-precision)") (TriggeredSeconds :type "Float (double-precision)") (InputAction :type "InputAction Object Reference" :default "/Game/PacManContent/Input/IA_Horizontal.IA_Horizontal"))
  (bind _gamemode (`self.GameMode`))
  ;[1 1 1] Input Action
  (:`Triggered`
    (set `self.Horizontal` ActionValue)
    ;[1 1 1] 플레이어가 버튼을 누르면 활성화
    (if (not (`/Game/PacManContent/BluePrint/BP_GameMode.IsStageStart` _gamemode)) :!label _label
      (set `/Game/PacManContent/BluePrint/BP_GameMode.IsStageStart` true _gamemode)))
  (:`Completed`
    (set `self.Horizontal` ActionValue)
    (goto _label)))

(event `EnhancedInput|/Game/PacManContent/Input/IA_Vertical`
  (params (ActionValue :type "Float (double-precision)") (ElapsedSeconds :type "Float (double-precision)") (TriggeredSeconds :type "Float (double-precision)") (InputAction :type "InputAction Object Reference" :default "/Game/PacManContent/Input/IA_Vertical.IA_Vertical"))
  ;[1 1 1] Input Action
  (:`Triggered`
    (set `self.Vertical` ActionValue)
    (goto _label))
  (:`Completed`
    (set `self.Vertical` ActionValue)
    (goto _label)))

(event `self.ReceiveBeginPlay`
  ;[1 1 1] Connect Enhanced Input System
  (`EnhancedInputSubsystemInterface.AddMappingContext` (pcsubsystem `EnhancedInputLocalPlayerSubsystem` (`GameplayStatics.GetPlayerController` 0)) "/Game/PacManContent/Input/IMC_PlayerInput.IMC_PlayerInput" 0 (struct))
  (bind _asbp_game_mode (cast `/Game/PacManContent/BluePrint/BP_GameMode` (`GameplayStatics.GetGameMode`))
    (:`then`
      (set `self.GameMode` _asbp_game_mode)
      (`self.Init`))
    (:`CastFailed`
      (`KismetSystemLibrary.PrintText` "게임모드가 없음"))))

(event `self.ReceiveActorBeginOverlap`
  (params (OtherActor :type "Actor Object Reference"))
  (if (`self.ActorHasTag` OtherActor "Item")
    (bind _asitem_spawner (cast `/Game/PacManContent/BluePrint/Item/ItemSpawner` OtherActor))
    (`/Game/PacManContent/BluePrint/Item/ItemSpawner.ItemEaten` _asitem_spawner)))

(event `self.ReceiveTick`
  (params (DeltaSeconds :type "Float (single-precision)"))
  (bind _gridoffset (`self.GridOffset`))
  (bind _gridoffset_2 (`self.GridOffset`))
  (`self.Set Next Dir`)
  (if (`/Game/PacManContent/BluePrint/BP_GameMode.IsStageStart` (`self.GameMode`))
    ;[1 1 1] 맨 처음 입력 세팅
    (if (== (`self.CurDir`) (`KismetMathLibrary.Vector_Zero`))
      (if (!= (`self.NextDir`) (`KismetMathLibrary.Vector_Zero`))
        (`self.SetCurDir`)
        (set `self.TargetPosition` (+ (`self.K2_GetActorLocation`) (* (`self.CurDir`) (`self.GridOffset`)))))
      (elif (< (`KismetMathLibrary.Vector_Distance` (`self.K2_GetActorLocation`) (`self.TargetPosition`)) 10.0)
        (`self.K2_SetActorLocation` (`KismetMathLibrary.MakeVector` (* (`KismetMathLibrary.Round` (/ (.x (`self.K2_GetActorLocation`)) _gridoffset_2)) _gridoffset) (* (`KismetMathLibrary.Round` (/ (.y (`self.K2_GetActorLocation`)) _gridoffset_2)) _gridoffset)))
        (`self.SetCurDir`)
        (bind _ishit (`self.Check Wall` (`self.CurDir`)))
        (if (not _ishit)
          ;[1 1 1] 타겟위치 재할당
          (set `self.TargetPosition` (+ (`self.K2_GetActorLocation`) (* (`self.CurDir`) (`self.GridOffset`))))
          (`self.K2_SetActorLocationAndRotation` (+ (`self.K2_GetActorLocation`) (* (* (`self.CurDir`) (`self.Speed`)) DeltaSeconds)) :!label _label_2))
        (else
          (goto _label_2))))))

(fn `Check Wall`
  (params (Dir :type "Vector Structure"))
  (returns (isHit :type Boolean))
  (bind _returnvalue (`self.K2_GetActorLocation`))
  (bind _returnvalue_2 (+ _returnvalue (* (`self.GridOffset`) Dir)))
  (`KismetSystemLibrary.DrawDebugLine` _returnvalue _returnvalue_2 (struct :`R` 0.189831 :`B` 1.0 :`A` 1.0))
  (bind _outhits (`KismetSystemLibrary.LineTraceMulti` _returnvalue _returnvalue_2 "TraceTypeQuery1" true))
  (for _array_element _outhits
    (bind (_bblockinghit _binitialoverlap _time _distance _location _impactpoint _normal _impactnormal _physmat _hitactor) (`GameplayStatics.BreakHitResult` _array_element))
    (if _bblockinghit
      (if (`self.ActorHasTag` _hitactor "Wall")
        (return true)
        (elif (`self.ActorHasTag` _hitactor "EntranceWall")
          (return true)))))
  (return false))

(fn `Init`
  (set `self.CurDir` (0.0 0.0 0.0))
  (set `self.NextDir` (0.0 0.0 0.0))
  (set `self.TargetPosition` (`self.K2_GetActorLocation`)))

(fn `Set Next Dir`
  (bind _vertical (`self.Vertical`))
  (bind _horizontal (`self.Horizontal`))
  (bind _returnvalue (`KismetMathLibrary.MakeVector` 0.0 _horizontal))
  (bind _returnvalue_2 (`KismetMathLibrary.MakeVector` _vertical))
  ;[1 1 1] Vertical이 유효한지 체크하고 그렇지 않다면 horizontal로 넘어감
  (if (== _vertical 0.0)
    ;[1 1 1] horizontal의 유효성 체크
    (if (== _horizontal 0.0)
      _
      (elif (not (== _returnvalue (`self.CurDir`)))
        (set `self.NextDir` _returnvalue)))
    (elif (not (== _returnvalue_2 (`self.CurDir`)))
      (set `self.NextDir` _returnvalue_2))))

(fn `SetCurDir`
  (bind _nextdir (`self.NextDir`))
  ;[1 1 1] nextDir 방향에 벽이있는지 체크
  (bind _ishit (`self.Check Wall` _nextdir))
  (if (not _ishit)
    ;[1 1 1] 현재 방향과 입력방향이 다르다면 현재방향을 업데이트
    (if (!= (`self.CurDir`) _nextdir)
      (set `self.CurDir` _nextdir))))

(fn `SetLocationToSpawnPos`
  (bind _returnvalue (`GameplayStatics.GetActorOfClass` "/Script/Engine.PlayerStart"))
  (`self.K2_SetActorLocation` (`self.K2_GetActorLocation` _returnvalue)))

(fn `UserConstructionScript`
  (`parent.UserConstructionScript`))