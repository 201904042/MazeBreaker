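; ItemBase is a base Blueprint for maze items that spin in place and can be eaten.
; BeginPlay caches the BP_GameMode reference, and Tick adds a small yaw rotation to RealMesh every frame.
; SetItemSpawner stores the spawner that owns the item.
; ItemEaten prints a debug message and tells that spawner to deactivate the item through UnActiveItem.
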(event `self.ReceiveBeginPlay`
  (bind _returnvalue (`GameplayStatics.GetActorOfClass` "/Game/MazeContent/BluePrint/BP_GameMode.BP_GameMode_C"))
  (set `self.GameMode` _returnvalue))

(event `self.ReceiveTick`
  (params (DeltaSeconds :type "Float (single-precision)"))
  (`SceneComponent.K2_AddLocalRotation` (`self.RealMesh`) (`KismetMathLibrary.MakeRotator` 0.0 0.0 1.0) false false))

(fn `ItemEaten`
  (`KismetSystemLibrary.PrintString` "아이템 작용")
  (`/Game/MazeContent/BluePrint/Item/ItemSpawner.UnActiveItem` (`self.ItemSpawner`)))

(fn `SetItemSpawner`
  (params (`new spawn` :type "/Game/MazeContent/BluePrint/Item/ItemSpawner Object Reference"))
  (set `self.ItemSpawner` `new spawn`))

(fn `UserConstructionScript`)