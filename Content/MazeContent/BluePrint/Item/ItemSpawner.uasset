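; Item spawn point actor for the maze game that creates a pickup at its spawn position component on request.
; SpawnItem marks the spawner active and switches on the requested type to spawn a crystal, EMP, boost or gun.
; Each spawned item is cast to ItemBase and handed a reference back to this spawner.
; UnActiveItem clears the active flag, and BeginPlay caches the game mode.
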(event `self.ReceiveBeginPlay`
  (bind _returnvalue (`GameplayStatics.GetActorOfClass` "/Game/MazeContent/BluePrint/BP_GameMode.BP_GameMode_C"))
  (set `self.GameMode` _returnvalue))

(fn `SpawnItem`
  (params (NewParam :type "/Game/MazeContent/BluePrint/Item/E_ItemType Enum" :default "NewEnumerator0"))
  (bind _returnvalue (`SceneComponent.K2_GetComponentToWorld` (`self.ItemSpawnPos`)))
  (set `self.ItemActive` true)
  (switch `/Game/MazeContent/BluePrint/Item/E_ItemType` NewParam
    (:`NewEnumerator0`
      (bind _returnvalue_2 (`|SpawnActorFromClass` "/Game/MazeContent/BluePrint/Item/BP_Crystal.BP_Crystal_C" _returnvalue "Undefined" "OverrideRootScale" null null))
      (bind _asitem_base (cast `/Game/MazeContent/BluePrint/Item/ItemBase` _returnvalue_2))
      (`/Game/MazeContent/BluePrint/Item/ItemBase.SetItemSpawner` _asitem_base self))
    (:`NewEnumerator1`
      (bind _returnvalue_3 (`|SpawnActorFromClass` "/Game/MazeContent/BluePrint/Item/BP_EMP.BP_EMP_C" _returnvalue "Undefined" "OverrideRootScale" null null))
      (bind _asitem_base_2 (cast `/Game/MazeContent/BluePrint/Item/ItemBase` _returnvalue_3))
      (`/Game/MazeContent/BluePrint/Item/ItemBase.SetItemSpawner` _asitem_base_2 self))
    (:`NewEnumerator2`
      (bind _returnvalue_4 (`|SpawnActorFromClass` "/Game/MazeContent/BluePrint/Item/BP_Boost.BP_Boost_C" _returnvalue "Undefined" "OverrideRootScale" null null))
      (bind _asitem_base_3 (cast `/Game/MazeContent/BluePrint/Item/ItemBase` _returnvalue_4))
      (`/Game/MazeContent/BluePrint/Item/ItemBase.SetItemSpawner` _asitem_base_3 self))
    (:`NewEnumerator3`
      (bind _returnvalue_5 (`|SpawnActorFromClass` "/Game/MazeContent/BluePrint/Item/BP_Gun.BP_Gun_C" _returnvalue "Undefined" "OverrideRootScale" null null))
      (bind _asitem_base_4 (cast `/Game/MazeContent/BluePrint/Item/ItemBase` _returnvalue_5))
      (`/Game/MazeContent/BluePrint/Item/ItemBase.SetItemSpawner` _asitem_base_4 self))))

(fn `UnActiveItem`
  (set `self.ItemActive` false))

(fn `UserConstructionScript`)