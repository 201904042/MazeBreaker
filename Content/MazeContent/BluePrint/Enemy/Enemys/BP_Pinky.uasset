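; BP_Pinky is the Pinky maze enemy, a child Blueprint that overrides the parent's chase targeting, animation and state hooks.
; Beyond a grid-scaled distance it targets cells ahead of the player's facing to ambush, otherwise the player's position, with optional debug circles.
; ChangeAnim assigns the BullSquid anim Blueprint and passes it the state.
; ChangeState plays the movement sound in one state and stops it in all others.
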(event `self.ReceiveBeginPlay`
  (`parent.ReceiveBeginPlay`))

(fn `ChangeAnim`
  (params (state :type "/Game/MazeContent/BluePrint/Enemy/BP_EnemyState Enum" :default "NewEnumerator0"))
  (bind _enemymesh (`self.EnemyMesh`))
  (`parent.ChangeAnim` state)
  (`SkeletalMeshComponent.SetAnimInstanceClass` _enemymesh "/Game/MazeContent/Animation/ABP_BullSquid.ABP_BullSquid_C")
  (bind _asabp_bull_squid (cast `/Game/MazeContent/Animation/ABP_BullSquid` (`SkeletalMeshComponent.GetAnimInstance` _enemymesh))
    (:`then`
      (set `/Game/MazeContent/Animation/ABP_BullSquid.curState` state _asabp_bull_squid))
    (:`CastFailed`
      (`KismetSystemLibrary.PrintString` "애니메이션 로드 실패"))))

(fn `ChangeState`
  (params (ChangeState :type "/Game/MazeContent/BluePrint/Enemy/BP_EnemyState Enum" :default "NewEnumerator0"))
  (bind _movesound (`self.MoveSound`))
  (`parent.ChangeState` ChangeState)
  (if (`|EnumEquality` ChangeState "NewEnumerator0")
    (`AudioComponent.Play` _movesound 0.0)
    (else
      (`AudioComponent.Stop` _movesound))))

(fn `SetTargetInChase`
  (returns (targetPos :type "Vector Structure"))
  (bind _player (`self.Player`))
  (bind _returnvalue (* (`self.GetActorForwardVector` _player) (`self.DefaultGridSize`)))
  (`parent.SetTargetInChase`)
  (if (> (`KismetMathLibrary.Vector_Distance` (`self.K2_GetActorLocation` (`self.Player`)) (`self.K2_GetActorLocation`)) (* (`self.PinkyChaseValue`) (`self.DefaultGridSize`)))
    (bind _output_get (set `self.TargetPosition` (+ (* _returnvalue (`self.PinkyChaseValue`)) (+ _returnvalue (`self.K2_GetActorLocation` _player)))))
    (if (`/Game/MazeContent/BluePrint/BP_GameMode.IsActiveDebugLine` (`self.GameMode`))
      (`KismetSystemLibrary.DrawDebugCircle` _output_get 100.0 12 (`KismetMathLibrary.Conv_ColorToLinearColor` (`self.C_DebugColor`)) 0.5 10.0 (0.0 1.0 0.0) (1.0 0.0 0.0)))
    (return _output_get)
    (else
      (bind _output_get_2 (set `self.TargetPosition` (`self.K2_GetActorLocation` (`self.Player`))))
      (if (`/Game/MazeContent/BluePrint/BP_GameMode.IsActiveDebugLine` (`self.GameMode`))
        (`KismetSystemLibrary.DrawDebugCircle` _output_get_2 100.0 12 (`KismetMathLibrary.Conv_ColorToLinearColor` (`self.C_DebugColor`)) 0.5 10.0 (0.0 1.0 0.0) (1.0 0.0 0.0)))
      (return _output_get_2))))

(fn `UserConstructionScript`
  (`parent.UserConstructionScript`))