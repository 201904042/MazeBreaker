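; BP_Blinky is a maze enemy that directly targets the player in chase mode, with most behavior inherited from its parent class.
; Its chase-target override returns the player's current location and draws a debug circle there when the game mode's debug flag is on.
; Its animation override assigns the headless dog Animation Blueprint to the mesh on each state change, then passes the new state to that instance.
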(event `self.ReceiveBeginPlay`
  (`parent.ReceiveBeginPlay`))

(fn `ChangeAnim`
  (params (state :type "/Game/MazeContent/BluePrint/Enemy/BP_EnemyState Enum" :default "NewEnumerator0"))
  (bind _enemymesh (`self.EnemyMesh`))
  (`parent.ChangeAnim` state)
  (`SkeletalMeshComponent.SetAnimInstanceClass` _enemymesh "/Game/MazeContent/Animation/ABP_HeadlessDog.ABP_HeadlessDog_C")
  (bind _asabp_headless_dog (cast `/Game/MazeContent/Animation/ABP_HeadlessDog` (`SkeletalMeshComponent.GetAnimInstance` _enemymesh)))
  (set `/Game/MazeContent/Animation/ABP_HeadlessDog.CurState` state _asabp_headless_dog))

(fn `Init`
  (`parent.Init`))

(fn `SetTargetInChase`
  (returns (targetPos :type "Vector Structure"))
  (`parent.SetTargetInChase`)
  (bind _output_get (set `self.TargetPosition` (`self.K2_GetActorLocation` (`self.Player`))))
  (if (`/Game/MazeContent/BluePrint/BP_GameMode.IsActiveDebugLine` (`self.GameMode`))
    (`KismetSystemLibrary.DrawDebugCircle` _output_get 100.0 12 (`KismetMathLibrary.Conv_ColorToLinearColor` (`self.C_DebugColor`)) 0.5 10.0 (0.0 1.0 0.0) (1.0 0.0 0.0)))
  (return _output_get))

(fn `UserConstructionScript`
  (`parent.UserConstructionScript`))